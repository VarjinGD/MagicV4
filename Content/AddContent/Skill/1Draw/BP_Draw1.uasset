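; BP_Draw1 is a skill projectile that dashes the player character to whatever actor it hits.
; On hit it runs a timeline that stops the projectile and lerps the character toward that actor with a rising height and fixed X offset.
; When finished, it destroys itself, reveals the character's body and gear meshes, deactivates the dash Niagara effect and, if the move succeeded, switches from the follow camera to the other camera.
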(event Custom|2MoveCharacter%20Event
  (params (act :type Actor%20Object%20Reference))
  (bind _returnvalue (Game|GetPlayerCharacter 0))
  (Utilities|Casting|CastToMyThirdPersonCharacter _returnvalue)
  (Variables|Default|SetStartCurrentCharacter (Transformation|GetActorLocation _returnvalue))
  (Components|Timeline|SetPlayRate (Variables|Default|GetTimeline_1) 2.0)
  (bind _val (Timeline|Timeline_1 Play)
    (:Update
      (Variables|/Script/Engine.MovementComponent|SetVelocity (Variables|Default|GetProjectileMovement) "0, 0, 0")
      (bind _asmy_third_person_character (Utilities|Casting|CastToMyThirdPersonCharacter (Game|GetPlayerCharacter 0)))
      (bind _output_get (Variables|Default|SetAs%20My%20Third%20Person%20Character _asmy_third_person_character))
      (bind _returnvalue_2 (Transformation|SetActorLocation _output_get (- (+ (Math|Vector|Lerp(Vector) (Variables|Default|GetStartCurrentCharacter) (Transformation|GetActorLocation act) _val) (* "0,0.000000,90.000000" _val)) "150.000000,0.000000,0") false false))
      (Variables|Default|SetHit _returnvalue_2))
    (:Finished
      (Actor|DestroyActor)
      (Rendering|SetVisibility (Variables|/Script/Engine.Character|GetMesh (Variables|Default|GetAs%20My%20Third%20Person%20Character)) true false)
      (Components|Activation|Deactivate (Variables|/Game/ThirdPersonBP/Blueprints/MyThirdPersonCharacter.MyThirdPersonCharacter_C|GetDash_NiagaraEmitter_System (Variables|Default|GetAs%20My%20Third%20Person%20Character)))
      (if (Variables|Default|GetHit)
        (Components|Activation|SetActive (Variables|/Game/ThirdPersonBP/Blueprints/MyThirdPersonCharacter.MyThirdPersonCharacter_C|GetFollowCamera (Variables|Default|GetAs%20My%20Third%20Person%20Character)) false false)
        (Components|Activation|SetActive (Variables|/Game/ThirdPersonBP/Blueprints/MyThirdPersonCharacter.MyThirdPersonCharacter_C|GetCamera (Variables|Default|GetAs%20My%20Third%20Person%20Character)) true false)))))

(event EventBeginPlay
  (Variables|Default|SetDraw_Start%20Location (Transformation|GetWorldLocation (Variables|Default|GetSphere)))
  (Utilities|FlowControl|Delay 1.0))

(event Collision|EventActorBeginOverlap
  (params (OtherActor :type Actor%20Object%20Reference)))

(event EventTick
  (params (DeltaSeconds :type Float%20%28single-precision%29)))

(event Collision|EventHit
  (params (MyComp :type Primitive%20Component%20Object%20Reference) (Other :type Actor%20Object%20Reference) (OtherComp :type Primitive%20Component%20Object%20Reference) (bSelfMoved :type Boolean) (HitLocation :type Vector :default "0, 0, 0") (HitNormal :type Vector :default "0, 0, 0") (NormalImpulse :type Vector :default "0, 0, 0") (Hit :type Hit%20Result%20Structure%20%28by%20ref%29))
  (CallFunction|2MoveCharacterEvent Other))

(fn ConstructionScript)