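; BP_Hook is a hook projectile that flies out, then retracts to its launch point, dragging any actor it hits.
; It records its sphere's start location and retracts after a one-second delay or on Hit.
; Two timelines zero velocity and lerp sphere and hit actor from their current locations toward that point, with sphere collision disabled.
; Either timeline finishing destroys the hook; the pull prints a debug "Hello".
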(event Custom|HookMove%20Event
  (bind _sphere (Variables|Default|GetSphere))
  (bind _val (Timeline|Comeback Play)
    (:Update
      (Variables|/Script/Engine.MovementComponent|SetVelocity (Variables|Default|GetProjectileMovement) "0, 0, 0")
      (Transformation|SetWorldLocation _sphere (Math|Vector|Lerp(Vector) (Transformation|GetWorldLocation (Variables|Default|GetSphere)) (Variables|Default|GetStartLocation) _val) false false)
      (Collision|SetCollisionEnabled _sphere "NoCollision"))
    (:Finished
      (Actor|DestroyActor))))

(event Custom|MoveObject%20Event
  (params (Actor :type Actor%20Object%20Reference))
  (bind _val (Timeline|Timeline_0 Play)
    (:Update
      (Variables|/Script/Engine.MovementComponent|SetVelocity (Variables|Default|GetProjectileMovement) "0, 0, 0")
      (Transformation|SetActorLocation Actor (Math|Vector|Lerp(Vector) (Transformation|GetActorLocation Actor) (Variables|Default|GetStartLocation) _val) false false)
      (Development|PrintString "Hello"))
    (:Finished
      (Actor|DestroyActor))))

(event EventBeginPlay
  (Variables|Default|SetStartLocation (Transformation|GetWorldLocation (Variables|Default|GetSphere)))
  (Utilities|FlowControl|Delay 1.0)
  (CallFunction|HookMoveEvent))

(event Collision|EventActorBeginOverlap
  (params (OtherActor :type Actor%20Object%20Reference)))

(event EventTick
  (params (DeltaSeconds :type Float%20%28single-precision%29)))

(event Collision|EventHit
  (params (MyComp :type Primitive%20Component%20Object%20Reference) (Other :type Actor%20Object%20Reference) (OtherComp :type Primitive%20Component%20Object%20Reference) (bSelfMoved :type Boolean) (HitLocation :type Vector :default "0, 0, 0") (HitNormal :type Vector :default "0, 0, 0") (NormalImpulse :type Vector :default "0, 0, 0") (Hit :type Hit%20Result%20Structure%20%28by%20ref%29))
  (CallFunction|HookMoveEvent)
  (CallFunction|MoveObjectEvent Other))

(fn ConstructionScript)