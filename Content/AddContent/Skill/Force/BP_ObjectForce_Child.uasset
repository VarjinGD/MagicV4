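; BP_ObjectForce_Child is a child of a force skill object Blueprint that makes four of its components (A, A1, A2, A3) blink repeatedly.
; Tick runs the parent logic, then a DoOnce gates a delayed sequence that hides the components, shows them again after a longer pause, and resets the gate to loop.
; BeginPlay, overlap and construction add no logic of their own.
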(event EventBeginPlay
  (|CallParentFunction) ; This node is disabled and will not be called.\nDrag off pins to build functionality.
)

(event Collision|EventActorBeginOverlap
  (params (OtherActor :type Actor%20Object%20Reference))
  (|CallParentFunction OtherActor) ; This node is disabled and will not be called.\nDrag off pins to build functionality.
)

(event EventTick
  (params (DeltaSeconds :type Float%20%28single-precision%29))
  (bind _a1 (Variables|Default|Geta1))
  (|CallParentFunction DeltaSeconds)
  (Utilities|FlowControl|DoOnce false :!label _label
    (:Completed
      (Utilities|FlowControl|Delay 0.2)
      (Rendering|SetVisibility _a1 false false)
      (Utilities|FlowControl|Delay 1.0)
      (Rendering|SetVisibility _a1 true false)
      (goto _label Reset))))

(fn ConstructionScript
  (|CallParentFunction))